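; BP_Player is a player actor that moves and turns from input axes.
; Forward and Right inputs add local X and Y offsets scaled by Speed, without sweep collision or delta-time scaling.
; Each Tick adds an axis key value as local yaw, plus the negated current roll and pitch to counter tilt.
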(event `InputAxis|Forward`
  (params (AxisValue :type "Float (single-precision)"))
  (`self.K2_AddActorLocalOffset` (`KismetMathLibrary.MakeVector` (* AxisValue (`self.Speed`)))))

(event `InputAxis|Right`
  (params (AxisValue :type "Float (single-precision)"))
  (`self.K2_AddActorLocalOffset` (`KismetMathLibrary.MakeVector` 0.0 (* AxisValue (`self.Speed`)))))

(event `self.ReceiveTick`
  (params (DeltaSeconds :type "Float (single-precision)"))
  (`self.K2_AddActorLocalRotation` (`KismetMathLibrary.MakeRotator` (* (.roll (`self.K2_GetActorRotation`)) -1.0) (* (.pitch (`self.K2_GetActorRotation`)) -1.0) (`self.GetInputAxisKeyValue`))))

(fn `UserConstructionScript`)